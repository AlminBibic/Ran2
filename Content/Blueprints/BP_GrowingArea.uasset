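; BP_GrowingArea is an area actor that tracks hit stones to trigger flower growth.
; CountStones increments a counter, and Tick compares it with StonesToActivate, printing "Grow Flowers" every frame they are equal as a placeholder for the growth.
; The construction script sizes the GrowRadius box from the GrowRadiusExtent variable; no overlap logic uses it yet.
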(event Custom|CountStones
  ;[1 1 1] Count Stones that you hited
  (Variables|Default|SetStonesCount (+ (Variables|Default|GetStonesCount) 1)))

(event EventBeginPlay)

(event Collision|EventActorBeginOverlap
  (params (OtherActor :type Actor%20Object%20Reference)))

(event EventTick
  (params (DeltaSeconds :type Float%20%28single-precision%29))
  (if (== (Variables|Default|GetStonesCount) (Variables|Default|GetStonesToActivate))
    (Development|PrintString "Grow Flowers" true true "(R=0.000220,G=0.192708,B=0.000000,A=1.000000)")))

(fn ConstructionScript
  (Components|Box|SetBoxExtent (Variables|Default|GetGrowRadius) (Variables|Default|GetGrowRadiusExtent) true))