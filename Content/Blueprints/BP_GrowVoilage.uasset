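; BP_GrowVoilage is an actor whose static mesh grows once the player pawn enters its overlap sphere, likely for foliage.
; The construction script applies the configurable mesh and starting scale.
; The sphere overlap sets a StartGrow flag, which this graph never clears, so Tick keeps interpolating the mesh's world scale toward GrowScale at GrowSpeed using VInterpTo.
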(event OnComponentBeginOverlap(Sphere)
  (params (OverlappedComponent :type Primitive%20Component%20Object%20Reference) (OtherActor :type Actor%20Object%20Reference) (OtherComp :type Primitive%20Component%20Object%20Reference) (OtherBodyIndex :type Integer) (bFromSweep :type Boolean) (SweepResult :type Hit%20Result%20Structure%20%28by%20ref%29))
  ;[1 1 1] Grow
  (if (== OtherActor (Game|Player|GetPlayerPawn 0))
    (Variables|Default|SetStartGrow true)))

(event Custom|Grow
  ;[1 1 1] Grow
  (Transformation|SetWorldScale3D (Variables|Default|GetStaticMesh) (Math|Interpolation|VInterpTo (Transformation|GetWorldScale (Variables|Default|GetStaticMesh)) (Variables|Grow|GetGrowScale) (Variables|Default|GetDeltaSeconds) (Variables|Grow|GetGrowSpeed))))

(event EventTick
  (params (DeltaSeconds :type Float%20%28single-precision%29))
  (Variables|Default|SetDeltaSeconds DeltaSeconds)
  (Utilities|FlowControl|Sequence
    (:then_0
      (if (Variables|Default|GetStartGrow)
        (CallFunction|Grow)))))

(fn ConstructionScript
  (Transformation|SetWorldScale3D (Variables|Default|GetStaticMesh) (Variables|Grow|GetStartScale))
  (Components|StaticMesh|SetStaticMesh (Variables|Default|GetStaticMesh) (Variables|Mesh|GetMesh)))