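; Test actor that bobs its static mesh up and down over time.
; Each tick it adds a relative Z offset from the cosine of time since creation, scaled by delta seconds, producing a smooth sine oscillation without sweep.
; A disconnected rotate-around-Z calculation offset from the mesh's world location is left unused, and the construction script is empty.
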(event EventTick
  (params (DeltaSeconds :type Float%20%28single-precision%29))
  (Transformation|AddRelativeLocation (Variables|Default|GetStaticMesh) (* (Math|Vector|MakeVector 0.0 0.0 (* (Math|Trig|Cos(Radians) (Actor|GetGameTimeSinceCreation)) 5e+01)) DeltaSeconds) false false))

(fn ConstructionScript)