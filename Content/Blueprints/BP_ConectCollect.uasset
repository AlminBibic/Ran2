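; BP_ConectCollect is a collectible shrine that activates through the player's Watering and Pressed flags.
; Both sphere overlap events set Watering true; end overlap also resets a DoOnce that Tick enters while Watering is set.
; When the DoOnce passes with Pressed true, it destroys the sphere and increments CollectorCount in the BP_SaveVariables game instance.
; Activation also flips the mesh material's Switch parameter and spawns a puff effect.
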(event OnComponentEndOverlap(Sphere)
  (params (OverlappedComponent :type Primitive%20Component%20Object%20Reference) (OtherActor :type Actor%20Object%20Reference) (OtherComp :type Primitive%20Component%20Object%20Reference) (OtherBodyIndex :type Integer))
  (bind _returnvalue (Game|Player|GetPlayerPawn 0))
  (if (== OtherActor _returnvalue)
    (bind _asbp_player (Utilities|Casting|CastToBP_Player _returnvalue))
    (Variables|/Game/Blueprints/BP_Player.BP_Player_C|SetWatering? _asbp_player true)
    (Utilities|FlowControl|DoOnce false) ; enters at Reset
  ))

(event OnComponentBeginOverlap(Sphere)
  (params (OverlappedComponent :type Primitive%20Component%20Object%20Reference) (OtherActor :type Actor%20Object%20Reference) (OtherComp :type Primitive%20Component%20Object%20Reference) (OtherBodyIndex :type Integer) (bFromSweep :type Boolean) (SweepResult :type Hit%20Result%20Structure%20%28by%20ref%29))
  (bind _returnvalue (Game|Player|GetPlayerPawn 0))
  (if (== OtherActor _returnvalue)
    (bind _asbp_player (Utilities|Casting|CastToBP_Player _returnvalue))
    (Variables|/Game/Blueprints/BP_Player.BP_Player_C|SetWatering? _asbp_player true)))

(event Custom|Collect
  ;[1 1 1] Collect
  (Components|DestroyComponent (Variables|Default|GetSphere))
  (bind _asbp_save_variables (Utilities|Casting|CastToBP_SaveVariables (Game|GetGameInstance)))
  (Variables|/Game/Blueprints/BP_SaveVariables.BP_SaveVariables_C|SetCollectorCount _asbp_save_variables (+ (Variables|/Game/Blueprints/BP_SaveVariables.BP_SaveVariables_C|GetCollectorCount _asbp_save_variables) 1)))

(event Custom|ShrineActivate
  (Rendering|Material|SetScalarParameterValueonMaterials (Variables|Default|GetStaticMesh) "Switch" 1.0)
  (Effects|SpawnEmitteratLocation "/Game/Particles/Flowers/P_Puff.P_Puff" (Transformation|GetWorldLocation (Variables|Default|GetStaticMesh)) "0, 0, 0" "7.000000,7.000000,7.000000" false))

(event EventTick
  (params (DeltaSeconds :type Float%20%28single-precision%29))
  (bind _returnvalue (Game|Player|GetPlayerPawn 0))
  (bind _asbp_player (Utilities|Casting|CastToBP_Player _returnvalue))
  (if (Variables|/Game/Blueprints/BP_Player.BP_Player_C|GetWatering? _asbp_player)
    (Utilities|FlowControl|DoOnce false
      (:Completed
        (bind _asbp_player_2 (Utilities|Casting|CastToBP_Player _returnvalue))
        (if (Variables|/Game/Blueprints/BP_Player.BP_Player_C|GetPressed _asbp_player_2)
          (CallFunction|Collect)
          (CallFunction|ShrineActivate))))))

(fn ConstructionScript)