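; BP_Scrifice is a sacrifice spot where the player places a carried offering.
; A sphere's overlap events set a flag while the player pawn is inside.
; Each Tick while overlapping, it checks BP_Player's Pressed and IsOffering flags, then reveals the hidden Offering component, destroys the player's PickUpActor component and prints a debug message.
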(event OnComponentBeginOverlap(Sphere)
  (params (OverlappedComponent :type Primitive%20Component%20Object%20Reference) (OtherActor :type Actor%20Object%20Reference) (OtherComp :type Primitive%20Component%20Object%20Reference) (OtherBodyIndex :type Integer) (bFromSweep :type Boolean) (SweepResult :type Hit%20Result%20Structure%20%28by%20ref%29))
  (if (== OtherActor (Game|Player|GetPlayerPawn 0))
    (Variables|Default|SetIsOverlapping true)))

(event OnComponentEndOverlap(Sphere)
  (params (OverlappedComponent :type Primitive%20Component%20Object%20Reference) (OtherActor :type Actor%20Object%20Reference) (OtherComp :type Primitive%20Component%20Object%20Reference) (OtherBodyIndex :type Integer))
  (if (== OtherActor (Game|Player|GetPlayerPawn 0))
    (Variables|Default|SetIsOverlapping false)))

(event EventTick
  (params (DeltaSeconds :type Float%20%28single-precision%29))
  (if (Variables|Default|GetIsOverlapping)
    (bind _asbp_player (Utilities|Casting|CastToBP_Player (Game|Player|GetPlayerPawn 0)))
    (if (Variables|/Game/Blueprints/Player/BP_Player.BP_Player_C|GetPressed _asbp_player)
      (if (Variables|/Game/Blueprints/Player/BP_Player.BP_Player_C|GetIsOffering _asbp_player)
        (Development|SetHiddeninGame (Variables|Default|GetOffering) false false)
        (Components|DestroyComponent (Variables|/Game/Blueprints/Player/BP_Player.BP_Player_C|GetPickUpActor _asbp_player))
        (Development|PrintString "Offering placed")))))

(fn ConstructionScript)