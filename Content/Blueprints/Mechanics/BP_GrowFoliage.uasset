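; Foliage actor that grows its static mesh once the player pawn enters its sphere, with a one-time particle burst.
; Tick interpolates world scale either straight to a target or, in advanced mode, in two stages using height and width targets.
; Growth can optionally increment a referenced altar's counter once, as soon as it starts.
; The construction script applies the configurable mesh and starting scale.
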(event OnComponentBeginOverlap(Sphere)
  (params (OverlappedComponent :type Primitive%20Component%20Object%20Reference) (OtherActor :type Actor%20Object%20Reference) (OtherComp :type Primitive%20Component%20Object%20Reference) (OtherBodyIndex :type Integer) (bFromSweep :type Boolean) (SweepResult :type Hit%20Result%20Structure%20%28by%20ref%29))
  ;[1 1 1] Grow
  (if (== OtherActor (Game|Player|GetPlayerPawn 0))
    (Variables|Grow|SetStartGrow true)
    (CallFunction|SpawnParticle)))

(event Custom|GrowAdvance
  (bind _staticmesh (Variables|Default|GetStaticMesh))
  (bind _returnvalue (Transformation|GetWorldScale _staticmesh))
  ;[1 1 1] Grow
  (Utilities|FlowControl|Sequence
    (:then_0
      (if (not (Variables|Grow|GetStopGrowH))
        (Transformation|SetWorldScale3D (Variables|Default|GetStaticMesh) (Math|Interpolation|VInterpTo _returnvalue (Variables|Grow|GetGrowScaleH) (Variables|Default|GetDeltaSeconds) (Variables|Grow|GetGrowSpeed)))))
    (:then_1
      (if (Math|Vector|Equal(Vector) _returnvalue (Variables|Grow|GetGrowScaleH) 1.0)
        (Variables|Grow|SetStartGrowW true)))
    (:then_2
      (if (Variables|Grow|GetStartGrowW)
        (Transformation|SetWorldScale3D (Variables|Default|GetStaticMesh) (Math|Interpolation|VInterpTo _returnvalue (Variables|Grow|GetGrowScaleW) (Variables|Default|GetDeltaSeconds) (Variables|Grow|GetGrowSpeed)))
        (Variables|Grow|SetStopGrowH true)))))

(event Custom|GrowNormal
  ;[1 1 1] Grow normal
  (Transformation|SetWorldScale3D (Variables|Default|GetStaticMesh) (Math|Interpolation|VInterpTo (Transformation|GetWorldScale (Variables|Default|GetStaticMesh)) (Variables|GrowNormal|GetGrowScale) (Variables|Default|GetDeltaSeconds) (Variables|Grow|GetGrowSpeed)))
  (CallFunction|SpawnParticle))

(event Custom|CountAltar
  (bind _bp_altarref (Variables|Altar|GetBP_AltarRef))
  ;[1 1 1] Count to Altar
  (Utilities|FlowControl|DoOnce false
    (:Completed
      (Variables|/Game/Blueprints/Mechanics/BP_Altar.BP_Altar_C|SetCurentCount _bp_altarref (+ (Variables|/Game/Blueprints/Mechanics/BP_Altar.BP_Altar_C|GetCurentCount _bp_altarref) 1)))))

(event Custom|SpawnParticle
  ;[1 1 1] Spawn Particle
  (Utilities|FlowControl|DoOnce false
    (:Completed
      (Effects|SpawnEmitteratLocation "/Game/StarterContent/Particles/P_Explosion.P_Explosion" (Transformation|GetWorldLocation (Variables|Default|GetStaticMesh)) "0, 0, 0" "7.000000,7.000000,7.000000"))))

(event EventTick
  (params (DeltaSeconds :type Float%20%28single-precision%29))
  (Variables|Default|SetDeltaSeconds DeltaSeconds)
  (Utilities|FlowControl|Sequence
    (:then_0
      (if (Variables|Grow|GetStartGrow)
        (if (Variables|Grow|GetScaleModeSwitch)
          (CallFunction|GrowAdvance)
          (if (Variables|Altar|GetCountToAltar)
            (CallFunction|CountAltar))
          (else
            (CallFunction|GrowNormal)
            (if (Variables|Altar|GetCountToAltar)
              (CallFunction|CountAltar))))))))

(fn ConstructionScript
  (Transformation|SetWorldScale3D (Variables|Default|GetStaticMesh) (Variables|Grow|GetStartScale))
  (Components|StaticMesh|SetStaticMesh (Variables|Default|GetStaticMesh) (Variables|Mesh|GetMesh)))