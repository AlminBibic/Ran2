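; BP_GrowingArea is an area that grows flowers once the player has hit enough stones.
; CountStones increments a counter, which Tick compares to the required total before firing the growth event through a DoOnce.
; Growth spawns BP_Growflower actors at random points within the GrowRadius box, sized in the construction script.
; A downward line trace then moves each Flower component to the hit location; a random height offset variant is unconnected.
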(event Custom|CountStones
  ;[1 1 1] Count Stones that you hited
  (Variables|Default|SetStonesCount (+ (Variables|Default|GetStonesCount) 1)))

(event Custom|GrowFlowersInArea
  (bind _growradius (Variables|Default|GetGrowRadius))
  (bind _boxextent (Variables|/Script/Engine.BoxComponent|GetBoxExtent _growradius))
  ;[0 1 0.165] TODO: Grow flower in the Area
  (for _index (range 0 (- (Variables|Default|GetFlowersToSpawn) 1))
    (bind _returnvalue (Game|SpawnActorfromClass "/Game/Blueprints/Mechanics/BP_Growflower.BP_Growflower_C" (Math|Transform|MakeTransform (Math|Random|RandomPointinBoundingBox (Transformation|GetWorldLocation _growradius) (Math|Vector|MakeVector (.x _boxextent) (.y _boxextent) 5e+01))) "AlwaysSpawn" 0 0))
    (bind _outhit (Collision|LineTraceByChannel (Transformation|GetWorldLocation (Variables|/Game/Blueprints/Mechanics/BP_Growflower.BP_Growflower_C|GetFlower _returnvalue)) (+ (Transformation|GetWorldLocation (Variables|/Game/Blueprints/Mechanics/BP_Growflower.BP_Growflower_C|GetFlower _returnvalue)) (* "0, 0,-1.000000" (Variables|Default|GetTraceDistance))) "TraceTypeQuery1" false 0 "None"))
    (Transformation|SetWorldLocation (Variables|/Game/Blueprints/Mechanics/BP_Growflower.BP_Growflower_C|GetFlower _returnvalue) (.Location (Collision|BreakHitResult _outhit)) false false)
    (Utilities|FlowControl|Delay 0.5)))

(event EventBeginPlay)

(event Collision|EventActorBeginOverlap
  (params (OtherActor :type Actor%20Object%20Reference)))

(event EventTick
  (params (DeltaSeconds :type Float%20%28single-precision%29))
  (if (== (Variables|Default|GetStonesCount) (Variables|Default|GetStonesToActivate))
    (Utilities|FlowControl|DoOnce false
      (:Completed
        (CallFunction|GrowFlowersinArea)
        (Development|PrintString "Grow Flowers" true true "(R=0.000220,G=0.192708,B=0.000000,A=1.000000)")))))

(fn ConstructionScript
  (Components|Box|SetBoxExtent (Variables|Default|GetGrowRadius) (Variables|Default|GetGrowRadiusExtent) true))