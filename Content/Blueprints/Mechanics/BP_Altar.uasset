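; Altar actor that rises from a start height once its count reaches the maximum, with a shake and a camera cutaway.
; Tick polls the count, which nothing here increments, then eases the mesh's Z upward with FInterpTo.
; Until it nears the end height, each tick also jitters X/Y and calls the camera switch, which disables input, blends to CameraSwitch, then returns view and input after a delay.
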(event Custom|AltarMoveUp
  (bind _staticmesh (Variables|Default|GetStaticMesh))
  (bind _relativelocation (Variables|/Script/Engine.SceneComponent|GetRelativeLocation _staticmesh))
  ;[1 1 1] Move the Altar up
  (Transformation|SetRelativeLocation _staticmesh (Math|Vector|MakeVector (.x _relativelocation) (.y _relativelocation) (Math|Interpolation|FInterpTo (.z _relativelocation) (Variables|Altar|GetEndZLocation) (Variables|Default|GetDeltaSeconds) (Variables|Altar|GetMoveUpSpeed))) false false))

(event Custom|Shake
  (bind _staticmesh (Variables|Default|GetStaticMesh))
  ;[1 1 1] Shake the Altar when moving up
  (Transformation|SetRelativeLocation _staticmesh (Math|Vector|MakeVector (Math|Random|RandomFloatinRange 0.0 2.0) (Math|Random|RandomFloatinRange 0.0 3.0) (.z (Variables|/Script/Engine.SceneComponent|GetRelativeLocation _staticmesh))) false false))

(event Custom|SwitchCamera
  ;[1 1 1] Switch camera when Altar moving up
  (Input|DisableInput (Game|GetPlayerController 0))
  (Game|Player|SetViewTargetwithBlend (Game|GetPlayerController 0) (Variables|Camera|GetCameraSwitch) (Variables|Camera|GetBlendTime) "VTBlend_Linear" 1.0 false)
  (Utilities|FlowControl|Delay (+ (Variables|Camera|GetBlendTime) (Variables|Camera|GetDelayToPlayer)))
  (Game|Player|SetViewTargetwithBlend (Game|GetPlayerController 0) (Game|Player|GetPlayerPawn 0) (Variables|Camera|GetBlendTime) "VTBlend_Linear" 1.0 false)
  (Input|EnableInput (Game|GetPlayerController 0)))

(event Custom|CheckCount
  ;[1 1 1] Check count
  (if (== (Variables|Altar|GetCurentCount) (Variables|Altar|GetMaxCount))
    (Variables|Altar|SetStartMoving true)))

(event EventBeginPlay
  (Utilities|FlowControl|Delay 3.0))

(event EventTick
  (params (DeltaSeconds :type Float%20%28single-precision%29))
  (Variables|Default|SetDeltaSeconds DeltaSeconds)
  (Utilities|FlowControl|Sequence
    (:then_0
      (if (Variables|Altar|GetStartMoving)
        (CallFunction|AltarMoveUp)
        (if (Variables|Altar|GetIsShaking)
          (CallFunction|Shake)
          (CallFunction|SwitchCamera))))
    (:then_1
      (if (Math|Float|NearlyEqual(Float) (.z (Variables|/Script/Engine.SceneComponent|GetRelativeLocation (Variables|Default|GetStaticMesh))) (Variables|Altar|GetEndZLocation) 15.0)
        (Variables|Altar|SetIsShaking false)))
    (:then_2
      (CallFunction|CheckCount))))

(fn ConstructionScript
  (bind _staticmesh (Variables|Default|GetStaticMesh))
  (bind _relativelocation (Variables|/Script/Engine.SceneComponent|GetRelativeLocation _staticmesh))
  (Transformation|SetRelativeLocation _staticmesh (Math|Vector|MakeVector (.x _relativelocation) (.y _relativelocation) (Variables|Altar|GetStartZLocation)) false false))