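; BP_GuidLight is a hovering guide light that leads the player along a series of points, then flies to a final destination.
; Overlapping its sphere starts interpolated flight to the next point, where it snaps on arrival and advances the index.
; Once the index equals StoneCount and the player is near, it flies to TargetPoint while a one-time camera blend to itself temporarily disables input and hides the player's particles.
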(event OnComponentBeginOverlap(Sphere)
  (params (OverlappedComponent :type Primitive%20Component%20Object%20Reference) (OtherActor :type Actor%20Object%20Reference) (OtherComp :type Primitive%20Component%20Object%20Reference) (OtherBodyIndex :type Integer) (bFromSweep :type Boolean) (SweepResult :type Hit%20Result%20Structure%20%28by%20ref%29))
  (if (== OtherActor (Game|Player|GetPlayerPawn 0))
    (Variables|Default|SetFly true)
    (Utilities|FlowControl|DoOnce false) ; enters at Reset
  ))

(event Custom|FlyToEnd
  (bind _guidlight (Variables|Default|GetGuidLight))
  (bind _targetpoint (Variables|Default|GetTargetPoint))
  (Utilities|IsValid _targetpoint
    (:Is%20Valid
      (Transformation|SetWorldLocation _guidlight (Math|Interpolation|VInterpTo (Transformation|GetWorldLocation _guidlight) (Transformation|GetWorldLocation (Variables|/Script/Engine.TargetPoint|GetSpriteComponent _targetpoint)) (Variables|Default|GetDeltaSeconds) (Variables|Default|GetFlySpeed)) false false)
      (Utilities|FlowControl|DoOnce false
        (:Completed
          (Input|DisableInput (Game|GetPlayerController 0))
          (bind _asbp_player (Utilities|Casting|CastToBP_Player (Game|Player|GetPlayerPawn 0)))
          (Rendering|SetVisibility (Variables|/Game/Blueprints/Player/BP_Player.BP_Player_C|GetParticleSystem _asbp_player) false false)
          (Game|Player|SetViewTargetwithBlend (Game|GetPlayerController 0) self (Variables|Default|GetCameraBlendTime) "VTBlend_Linear" 1.0 false)
          (Utilities|FlowControl|Delay (+ (Variables|Default|GetDelayToPlayer) (Variables|Default|GetCameraBlendTime)))
          (Game|Player|SetViewTargetwithBlend (Game|GetPlayerController 0) (Game|Player|GetPlayerPawn 0) (Variables|Default|GetCameraBlendTime) "VTBlend_Linear" 1.0 false)
          (Input|EnableInput (Game|GetPlayerController 0))
          (Rendering|SetVisibility (Variables|/Game/Blueprints/Player/BP_Player.BP_Player_C|GetParticleSystem _asbp_player) true false))))))

(event Custom|FlyToNextPoint
  (bind _pointrefs (Variables|Default|GetPointRefs))
  (bind _index (Variables|Default|GetIndex))
  (bind _guidlight (Variables|Default|GetGuidLight))
  (bind _output (Utilities|Array|Get(acopy) _pointrefs _index))
  (bind _guidlightpoint (Variables|/Game/Blueprints/Mechanics/BP_GlowStone.BP_GlowStone_C|GetGuidLightPoint _output))
  (Utilities|IsValid _guidlightpoint
    (:Is%20Valid
      (Transformation|SetWorldLocation _guidlight (Math|Interpolation|VInterpTo (Transformation|GetWorldLocation _guidlight) (Transformation|GetWorldLocation _guidlightpoint) (Variables|Default|GetDeltaSeconds) (Variables|Default|GetFlySpeed)) false false))))

(event Custom|CheckDistance
  (Utilities|IsValid (Variables|/Game/Blueprints/Mechanics/BP_GlowStone.BP_GlowStone_C|GetGuidLightPoint (Utilities|Array|Get(acopy) (Variables|Default|GetPointRefs) (Variables|Default|GetIndex)))
    (:Is%20Valid
      (if (Math|Vector|Equal(Vector) (Transformation|GetWorldLocation (Variables|Default|GetGuidLight)) (Transformation|GetWorldLocation (Variables|/Game/Blueprints/Mechanics/BP_GlowStone.BP_GlowStone_C|GetGuidLightPoint (Utilities|Array|Get(acopy) (Variables|Default|GetPointRefs) (Variables|Default|GetIndex)))) 3e+02)
        (Utilities|IsValid (Variables|/Game/Blueprints/Mechanics/BP_GlowStone.BP_GlowStone_C|GetGuidLightPoint (Utilities|Array|Get(acopy) (Variables|Default|GetPointRefs) (Variables|Default|GetIndex)))
          (:Is%20Valid
            (Transformation|SetWorldLocation (Variables|Default|GetGuidLight) (Transformation|GetWorldLocation (Variables|/Game/Blueprints/Mechanics/BP_GlowStone.BP_GlowStone_C|GetGuidLightPoint (Utilities|Array|Get(acopy) (Variables|Default|GetPointRefs) (Variables|Default|GetIndex)))) false false)
            (Variables|Default|SetFly false)
            (Utilities|FlowControl|DoOnce false
              (:Completed
                (Variables|Default|SetIndex (+ (Variables|Default|GetIndex) 1))))))))))

(event Custom|Hover
  (bind _returnvalue (Actor|GetGameTimeSinceCreation))
  (bind _guidlight (Variables|Default|GetGuidLight))
  (bind _deltaseconds (Variables|Default|GetDeltaSeconds))
  (bind _returnvalue_2 (Math|Trig|Cos(Radians) _returnvalue))
  (bind _returnvalue_3 (* _returnvalue_2 2e+01))
  (bind _returnvalue_4 (* _returnvalue_2 5e+01))
  (bind _returnvalue_5 (* _returnvalue_2 25.0))
  (bind _returnvalue_6 (* (Math|Vector|MakeVector _returnvalue_4 _returnvalue_5 _returnvalue_3) _deltaseconds))
  (Transformation|AddRelativeLocation _guidlight (* (Math|Vector|MakeVector (* _returnvalue_2 8e+01) (* _returnvalue_2 -3e+01) (* _returnvalue_2 35.0)) (Variables|Default|GetDeltaSeconds)) false false)
  (Transformation|AddRelativeRotation _guidlight (Math|Rotator|MakeRotator (.x _returnvalue_6) (.y _returnvalue_6) (.z _returnvalue_6)) false false))

(event EventTick
  (params (DeltaSeconds :type Float%20%28single-precision%29))
  (Variables|Default|SetDeltaSeconds DeltaSeconds)
  (Utilities|FlowControl|Sequence
    (:then_0
      (CallFunction|CheckDistance))
    (:then_1
      (if (Variables|Default|GetFly)
        (CallFunction|FlytoNextPoint)))
    (:then_2
      (CallFunction|Hover))
    (:then_3
      (if (<= (Math|Vector|VectorLength (- (Transformation|GetWorldLocation (Variables|Default|GetGuidLight)) (Transformation|GetWorldLocation (Variables|/Game/Blueprints/Player/BP_Player.BP_Player_C|GetHead (Variables|Default|GetPlayerRef))))) 5e+02)
        (if (== (Variables|Default|GetIndex) (Variables|Default|GetStoneCount))
          (Utilities|FlowControl|DoOnce false
            (:Completed
              (Variables|Default|SetFlyToDestination true))))))
    (:then_4
      (if (Variables|Default|GetFlyToDestination)
        (CallFunction|FlytoEnd)))))

(fn ConstructionScript)