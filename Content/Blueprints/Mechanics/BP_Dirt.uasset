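; BP_Dirt is a cluster of four destructible rocks that the player smashes to make a static mesh available for pickup.
; Tick permanently arms the rocks once BP_Player's velocity passes a threshold, so sphere overlaps then apply upward-impulse damage and remove that trigger.
; Each break increments a counter; when all four are broken, overlapping the mesh registers it as BP_Player's pickup target, and leaving clears the in-object flag.
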(event OnComponentBeginOverlap(Sphere)
  (params (OverlappedComponent :type Primitive%20Component%20Object%20Reference) (OtherActor :type Actor%20Object%20Reference) (OtherComp :type Primitive%20Component%20Object%20Reference) (OtherBodyIndex :type Integer) (bFromSweep :type Boolean) (SweepResult :type Hit%20Result%20Structure%20%28by%20ref%29))
  (bind _sphere (Variables|Default|GetSphere))
  (bind _sm_rock_dm (Variables|Default|GetSM_Rock_DM))
  (if (== OtherActor (Game|Player|GetPlayerPawn 0))
    (if (Variables|Default|GetDestructible)
      (CallFunction|Count)
      (Class|DestructibleComponent|ApplyDamage _sm_rock_dm 2.0 (Transformation|GetWorldLocation _sm_rock_dm) (Math|Vector|GetUpVector _sm_rock_dm) (Variables|Default|GetDestroyPower))
      (Utilities|IsValid _sphere
        (:Is%20Valid
          (Components|DestroyComponent _sphere))))))

(event OnComponentBeginOverlap(Sphere1)
  (params (OverlappedComponent :type Primitive%20Component%20Object%20Reference) (OtherActor :type Actor%20Object%20Reference) (OtherComp :type Primitive%20Component%20Object%20Reference) (OtherBodyIndex :type Integer) (bFromSweep :type Boolean) (SweepResult :type Hit%20Result%20Structure%20%28by%20ref%29))
  (bind _sphere1 (Variables|Default|GetSphere1))
  (bind _sm_rock_dm1 (Variables|Default|GetSM_Rock_DM1))
  (if (== OtherActor (Game|Player|GetPlayerPawn 0))
    (if (Variables|Default|GetDestructible)
      (CallFunction|Count)
      (Class|DestructibleComponent|ApplyDamage _sm_rock_dm1 2.0 (Transformation|GetWorldLocation _sm_rock_dm1) (Math|Vector|GetUpVector _sm_rock_dm1) (Variables|Default|GetDestroyPower))
      (Utilities|IsValid _sphere1
        (:Is%20Valid
          (Components|DestroyComponent _sphere1))))))

(event OnComponentBeginOverlap(Sphere3)
  (params (OverlappedComponent :type Primitive%20Component%20Object%20Reference) (OtherActor :type Actor%20Object%20Reference) (OtherComp :type Primitive%20Component%20Object%20Reference) (OtherBodyIndex :type Integer) (bFromSweep :type Boolean) (SweepResult :type Hit%20Result%20Structure%20%28by%20ref%29))
  (bind _sm_rock_dm2 (Variables|Default|GetSM_Rock_DM2))
  (bind _sphere3 (Variables|Default|GetSphere3))
  (if (== OtherActor (Game|Player|GetPlayerPawn 0))
    (if (Variables|Default|GetDestructible)
      (CallFunction|Count)
      (Class|DestructibleComponent|ApplyDamage _sm_rock_dm2 2.0 (Transformation|GetWorldLocation _sm_rock_dm2) (Math|Vector|GetUpVector _sm_rock_dm2) (Variables|Default|GetDestroyPower))
      (Utilities|IsValid _sphere3
        (:Is%20Valid
          (Components|DestroyComponent _sphere3))))))

(event OnComponentBeginOverlap(Sphere2)
  (params (OverlappedComponent :type Primitive%20Component%20Object%20Reference) (OtherActor :type Actor%20Object%20Reference) (OtherComp :type Primitive%20Component%20Object%20Reference) (OtherBodyIndex :type Integer) (bFromSweep :type Boolean) (SweepResult :type Hit%20Result%20Structure%20%28by%20ref%29))
  (bind _sphere2 (Variables|Default|GetSphere2))
  (bind _sm_rock_dm3 (Variables|Default|GetSM_Rock_DM3))
  (if (== OtherActor (Game|Player|GetPlayerPawn 0))
    (if (Variables|Default|GetDestructible)
      (CallFunction|Count)
      (Class|DestructibleComponent|ApplyDamage _sm_rock_dm3 2.0 (Transformation|GetWorldLocation _sm_rock_dm3) (Math|Vector|GetUpVector _sm_rock_dm3) (Variables|Default|GetDestroyPower))
      (Utilities|IsValid _sphere2
        (:Is%20Valid
          (Components|DestroyComponent _sphere2))))))

(event OnComponentBeginOverlap(StaticMesh)
  (params (OverlappedComponent :type Primitive%20Component%20Object%20Reference) (OtherActor :type Actor%20Object%20Reference) (OtherComp :type Primitive%20Component%20Object%20Reference) (OtherBodyIndex :type Integer) (bFromSweep :type Boolean) (SweepResult :type Hit%20Result%20Structure%20%28by%20ref%29))
  (bind _returnvalue (Game|Player|GetPlayerPawn 0))
  (if (== OtherActor _returnvalue)
    (if (Variables|Default|GetCanPickup)
      (bind _asbp_player (Utilities|Casting|CastToBP_Player _returnvalue))
      (Variables|/Game/Blueprints/Player/BP_Player.BP_Player_C|SetInObject _asbp_player true)
      (Variables|/Game/Blueprints/Player/BP_Player.BP_Player_C|SetPickUpActor _asbp_player (Variables|Default|GetStaticMesh)))))

(event OnComponentEndOverlap(StaticMesh)
  (params (OverlappedComponent :type Primitive%20Component%20Object%20Reference) (OtherActor :type Actor%20Object%20Reference) (OtherComp :type Primitive%20Component%20Object%20Reference) (OtherBodyIndex :type Integer))
  (bind _returnvalue (Game|Player|GetPlayerPawn 0))
  (if (== OtherActor _returnvalue)
    (if (Variables|Default|GetCanPickup)
      (bind _asbp_player (Utilities|Casting|CastToBP_Player _returnvalue))
      (Variables|/Game/Blueprints/Player/BP_Player.BP_Player_C|SetInObject _asbp_player false))))

(event Custom|Count
  ;[1 1 1] Count index
  (Variables|Default|SetIndex (+ (Variables|Default|GetIndex) 1)))

(event EventTick
  (params (DeltaSeconds :type Float%20%28single-precision%29))
  (Utilities|FlowControl|Sequence
    (:then_0
      (bind _asbp_player (Utilities|Casting|CastToBP_Player (Game|Player|GetPlayerPawn 0)))
      (if (> (Variables|/Game/Blueprints/Player/BP_Player.BP_Player_C|GetPlayerVelocity _asbp_player) 7e+02)
        (Variables|Default|SetDestructible true)))
    (:then_1
      (if (== (Variables|Default|GetIndex) 4)
        (Variables|Default|SetCanPickup true)))))

(fn ConstructionScript)