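; Sacrifice point where the player, while carrying an offering, presses to place it, triggering a one-time camera cutaway.
; Sphere overlap gates a Tick poll of the player's pressed and offering state; DoOnce then reveals the Offering and destroys the carried pickup component.
; SwitchCamera hides the player's particles, blends to CameraSwitch, then after a delay starts blending back and restores the particles.
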(event OnComponentBeginOverlap(Sphere)
  (params (OverlappedComponent :type Primitive%20Component%20Object%20Reference) (OtherActor :type Actor%20Object%20Reference) (OtherComp :type Primitive%20Component%20Object%20Reference) (OtherBodyIndex :type Integer) (bFromSweep :type Boolean) (SweepResult :type Hit%20Result%20Structure%20%28by%20ref%29))
  (if (== OtherActor (Game|Player|GetPlayerPawn 0))
    (Variables|Default|SetIsOverlapping true)))

(event OnComponentEndOverlap(Sphere)
  (params (OverlappedComponent :type Primitive%20Component%20Object%20Reference) (OtherActor :type Actor%20Object%20Reference) (OtherComp :type Primitive%20Component%20Object%20Reference) (OtherBodyIndex :type Integer))
  (if (== OtherActor (Game|Player|GetPlayerPawn 0))
    (Variables|Default|SetIsOverlapping false)))

(event Custom|SwitchCamera
  (Input|DisableInput (Game|GetPlayerController 0))
  (bind _asbp_player (Utilities|Casting|CastToBP_Player (Game|Player|GetPlayerPawn 0)))
  (Rendering|SetVisibility (Variables|/Game/Blueprints/Player/BP_Player.BP_Player_C|GetParticleSystem _asbp_player) false false)
  (Game|Player|SetViewTargetwithBlend (Game|GetPlayerController 0) (Variables|CameraSwitch|GetCameraSwitch) (Variables|Default|GetCameraBlendTime) "VTBlend_Linear" 1.0 false)
  (Utilities|FlowControl|Delay (+ (Variables|Default|GetDelayToPlayer) (Variables|Default|GetCameraBlendTime)))
  (Game|Player|SetViewTargetwithBlend (Game|GetPlayerController 0) (Game|Player|GetPlayerPawn 0) (Variables|Default|GetCameraBlendTime) "VTBlend_Linear" 1.0 false)
  (Input|EnableInput (Game|GetPlayerController 0))
  (Rendering|SetVisibility (Variables|/Game/Blueprints/Player/BP_Player.BP_Player_C|GetParticleSystem _asbp_player) true false))

(event EventTick
  (params (DeltaSeconds :type Float%20%28single-precision%29))
  (if (Variables|Default|GetIsOverlapping)
    (bind _asbp_player (Utilities|Casting|CastToBP_Player (Game|Player|GetPlayerPawn 0)))
    (if (Variables|/Game/Blueprints/Player/BP_Player.BP_Player_C|GetPressed _asbp_player)
      (if (Variables|/Game/Blueprints/Player/BP_Player.BP_Player_C|GetIsOffering _asbp_player)
        (Utilities|FlowControl|DoOnce false
          (:Completed
            (Development|SetHiddeninGame (Variables|Default|GetOffering) false false)
            (Components|DestroyComponent (Variables|/Game/Blueprints/Player/BP_Player.BP_Player_C|GetPickUpActor _asbp_player))
            (CallFunction|SwitchCamera)
            (Development|PrintString "Offering placed")))))))

(fn ConstructionScript)