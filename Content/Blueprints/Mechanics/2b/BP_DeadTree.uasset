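; BP_DeadTree is an interactive dead tree that revives its ivy when the player presses input nearby.
; Two overlap volumes track the player, with the watering radius also toggling the player's watering permission.
; Once growing starts, Tick crossfades dried ivy to living ivy by stepping each material's Alpha parameter.
; While growing, overlapped and pickup-enabled, it sets BP_Player's offering state with Skul as the pickup actor.
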(event OnComponentBeginOverlap(Sphere)
  (params (OverlappedComponent :type Primitive%20Component%20Object%20Reference) (OtherActor :type Actor%20Object%20Reference) (OtherComp :type Primitive%20Component%20Object%20Reference) (OtherBodyIndex :type Integer) (bFromSweep :type Boolean) (SweepResult :type Hit%20Result%20Structure%20%28by%20ref%29))
  (if (== OtherActor (Game|Player|GetPlayerPawn 0))
    (Variables|Default|SetIsOverlapping true)))

(event OnComponentEndOverlap(Sphere)
  (params (OverlappedComponent :type Primitive%20Component%20Object%20Reference) (OtherActor :type Actor%20Object%20Reference) (OtherComp :type Primitive%20Component%20Object%20Reference) (OtherBodyIndex :type Integer))
  (if (== OtherActor (Game|Player|GetPlayerPawn 0))
    (Variables|Default|SetIsOverlapping false)
    (Variables|/Game/Blueprints/Player/BP_Player.BP_Player_C|SetInObject (stale EventTick _asbp_player) false)))

(event OnComponentBeginOverlap(Wateringradius)
  (params (OverlappedComponent :type Primitive%20Component%20Object%20Reference) (OtherActor :type Actor%20Object%20Reference) (OtherComp :type Primitive%20Component%20Object%20Reference) (OtherBodyIndex :type Integer) (bFromSweep :type Boolean) (SweepResult :type Hit%20Result%20Structure%20%28by%20ref%29))
  (if (== OtherActor (Game|Player|GetPlayerPawn 0))
    (Variables|Default|SetIsOverlapping true)
    (bind _asbp_player (Utilities|Casting|CastToBP_Player (Game|Player|GetPlayerPawn 0)))
    (Variables|/Game/Blueprints/Player/BP_Player.BP_Player_C|SetCanWattering _asbp_player true)))

(event OnComponentEndOverlap(Wateringradius)
  (params (OverlappedComponent :type Primitive%20Component%20Object%20Reference) (OtherActor :type Actor%20Object%20Reference) (OtherComp :type Primitive%20Component%20Object%20Reference) (OtherBodyIndex :type Integer))
  (if (== OtherActor (Game|Player|GetPlayerPawn 0))
    (Variables|Default|SetIsOverlapping false)
    (bind _asbp_player (Utilities|Casting|CastToBP_Player (Game|Player|GetPlayerPawn 0)))
    (Variables|/Game/Blueprints/Player/BP_Player.BP_Player_C|SetCanWattering _asbp_player false)))

(event Custom|Grow
  (bind _output_get (Variables|Default|SetDriedIvyAlpha (Math|Float|Clamp(Float) (- (Variables|Default|GetDriedIvyAlpha) 0.005))))
  (Rendering|Material|SetScalarParameterValueonMaterials (Variables|Default|GetDired_Ivy) "Alpha" _output_get)
  (bind _output_get_2 (Variables|Default|SetLivingIvyAlpha (Math|Float|Clamp(Float) (+ (Variables|Default|GetLivingIvyAlpha) 0.005))))
  (Rendering|Material|SetScalarParameterValueonMaterials (Variables|Default|GetLiving_Ivy) "Alpha" _output_get_2))

(event EventBeginPlay)

(event Collision|EventActorBeginOverlap
  (params (OtherActor :type Actor%20Object%20Reference)))

(event EventTick
  (params (DeltaSeconds :type Float%20%28single-precision%29))
  (Utilities|FlowControl|Sequence
    (:then_0
      (if (Variables|Default|GetIsGrowing)
        (CallFunction|Grow)))
    (:then_1
      (if (Variables|Default|GetIsGrowing)
        (if (Variables|Default|GetCanPickUp)
          (if (Variables|Default|GetIsOverlapping)
            (bind _asbp_player (Utilities|Casting|CastToBP_Player (Game|Player|GetPlayerPawn 0)))
            (Variables|/Game/Blueprints/Player/BP_Player.BP_Player_C|SetInObject _asbp_player true)
            (Variables|/Game/Blueprints/Player/BP_Player.BP_Player_C|SetPickUpActor _asbp_player (Variables|Default|GetSkul))
            (Variables|/Game/Blueprints/Player/BP_Player.BP_Player_C|SetIsOffering _asbp_player true)))))
    (:then_2
      (if (Variables|Default|GetIsOverlapping)
        (bind _asbp_player_2 (Utilities|Casting|CastToBP_Player (Game|Player|GetPlayerPawn 0)))
        (if (Variables|/Game/Blueprints/Player/BP_Player.BP_Player_C|GetPressed _asbp_player_2)
          (Variables|Default|SetIsGrowing true))))))

(fn ConstructionScript)