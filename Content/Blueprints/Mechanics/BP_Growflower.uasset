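; BP_Growflower is a flower actor that grows after spawning and vanishes when the player touches it.
; Construction picks a random material from an array for the Flower component.
; Tick scales the flower up by a fixed, frame-rate-dependent step until it reaches a clamped maximum size.
; Player pawn overlap with the Sphere spawns a puff emitter above the flower and destroys the actor, with no shrink animation.
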(event OnComponentBeginOverlap(Sphere)
  (params (OverlappedComponent :type Primitive%20Component%20Object%20Reference) (OtherActor :type Actor%20Object%20Reference) (OtherComp :type Primitive%20Component%20Object%20Reference) (OtherBodyIndex :type Integer) (bFromSweep :type Boolean) (SweepResult :type Hit%20Result%20Structure%20%28by%20ref%29))
  ;[1 1 1] Shrink and  Destroy Actor OnOverlap
  (if (== OtherActor (Game|Player|GetPlayerPawn 0))
    (CallFunction|DestroyFlower)))

(event Custom|Grow
  ;[1 1 1] Grow Flower
  (bind _output_get (Variables|Default|SetSize (Math|Float|Clamp(Float) (+ (Variables|Default|GetSize) 0.05) 0.0 1.5)))
  (Transformation|SetWorldScale3D (Variables|Default|GetFlower) (Math|Conversions|ToVector(Float) _output_get)))

(event Custom|DestroyFlower
  (bind _flower (Variables|Default|GetFlower))
  (bind _returnvalue (Transformation|GetWorldLocation _flower))
  ;[1 1 1] Destroy Flower
  (Effects|SpawnEmitteratLocation "/Game/Particles/Flowers/P_Puff.P_Puff" (Math|Vector|MakeVector (.x _returnvalue) (.y _returnvalue) (+ (.z _returnvalue) 2.5e+02)))
  (Utilities|IsValid self
    (:Is%20Valid
      (Actor|DestroyActor))))

(event EventBeginPlay)

(event EventTick
  (params (DeltaSeconds :type Float%20%28single-precision%29))
  (CallFunction|Grow))

(fn ConstructionScript
  (Rendering|Material|SetMaterial (Variables|Default|GetFlower) 0 (Utilities|Array|Get(acopy) (Variables|Default|GetMaterials) (Math|Random|RandomIntegerinRange 0 3))))