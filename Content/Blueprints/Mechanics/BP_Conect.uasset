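; Spline-path connect puzzle that activates a shrine once the player collects along the path and closes the connection.
; BeginPlay spawns collectors at spline points and builds spline meshes between them.
; Tick polls the GameInstance's CollectorCount, storing the player's head position at the first pickup and moving the closing overlap Sphere there after the last.
; Overlapping it lights the shrine, plays a camera blend, then grows flowers along the spline and sends the guide light onward.
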(event OnComponentBeginOverlap(Sphere)
  (params (OverlappedComponent :type Primitive%20Component%20Object%20Reference) (OtherActor :type Actor%20Object%20Reference) (OtherComp :type Primitive%20Component%20Object%20Reference) (OtherBodyIndex :type Integer) (bFromSweep :type Boolean) (SweepResult :type Hit%20Result%20Structure%20%28by%20ref%29))
  ;[1 1 1] Conected
  (if (== OtherActor (Game|Player|GetPlayerPawn 0))
    (Variables|Default|SetConected true)
    (Development|PrintString "Last Connected")))

(event Custom|ShrineActivate
  ;[1 1 1] ShrineActivate
  (Rendering|Material|SetScalarParameterValueonMaterials (Variables|Default|GetShrine) "Switch" 1.0)
  (Utilities|FlowControl|DoOnce false
    (:Completed
      (CallFunction|SwitchCamera))))

(event Custom|SpawnCollectorAlongSpline
  (bind _spline (Variables|Default|GetSpline))
  (bind _returnvalue (Spline|GetNumberOfSplinePoints _spline))
  ;[1 1 1] Spawn Collector along Spline
  (Variables|Default|SetIndex _returnvalue)
  (for _index (range 0 _returnvalue)
    (Game|SpawnActorfromClass "/Game/Blueprints/Mechanics/BP_ConectCollect.BP_ConectCollect_C" (Math|Transform|MakeTransform (Spline|GetLocationatSplinePoint _spline _index "World")) "AlwaysSpawn" 0 0)))

(event Custom|SpawnSplineMesh
  (bind _spline (Variables|Default|GetSpline))
  ;[1 1 1] Create SplineMesh
  (for _index (range 1 (Spline|GetNumberOfSplinePoints (Variables|Default|GetSpline)))
    (bind _returnvalue (AddComponent|AddSplineMeshComponent true))
    (Variables|Default|SetSPM _returnvalue)
    (SplineMesh|SetStartandEnd _returnvalue (.Location (Spline|GetLocationandTangentatSplinePoint _spline (- _index 1) "World")) (.Tangent (Spline|GetLocationandTangentatSplinePoint _spline (- _index 1) "World")) (.Location (Spline|GetLocationandTangentatSplinePoint _spline _index "World")) (.Tangent (Spline|GetLocationandTangentatSplinePoint _spline _index "World")) true :!class /Script/Engine.SplineMeshComponent)))

(event Custom|SwitchCamera
  ;[1 1 1] CameraSwitch
  (Input|DisableInput (Game|GetPlayerController 0))
  (bind _asbp_player (Utilities|Casting|CastToBP_Player (Game|Player|GetPlayerPawn 0)))
  (Rendering|SetVisibility (Variables|/Game/Blueprints/Player/BP_Player.BP_Player_C|GetParticleSystem _asbp_player) false false)
  (Game|Player|SetViewTargetwithBlend (Game|GetPlayerController 0) (Variables|Default|GetCameraSwitch) (Variables|Default|GetCameraBlendTime) "VTBlend_Linear" 1.0 false)
  (Utilities|FlowControl|Delay (+ (Variables|Default|GetDelayToPlayer) (Variables|Default|GetCameraBlendTime)))
  (Game|Player|SetViewTargetwithBlend (Game|GetPlayerController 0) (Game|Player|GetPlayerPawn 0) (Variables|Default|GetCameraBlendTime) "VTBlend_Linear" 1.0 false)
  (Input|EnableInput (Game|GetPlayerController 0))
  (Rendering|SetVisibility (Variables|/Game/Blueprints/Player/BP_Player.BP_Player_C|GetParticleSystem _asbp_player) true false))

(event Custom|SpawnFlowersAlongSpline
  (bind _spline (Variables|Default|GetSpline))
  (bind _spacing (Variables|Default|GetSpacing))
  (bind _guidlightref (Variables|Default|GetGuidLightRef))
  ;[1 1 1] SpawnFlowersAlongSpline
  (for _index (range 0 (.ReturnValue (Math|Float|Division(WholeandRemainder) (Spline|GetSplineLength _spline) _spacing)))
    (bind _returnvalue (Game|SpawnActorfromClass "/Game/Blueprints/Mechanics/BP_Growflower.BP_Growflower_C" (Math|Transform|MakeTransform (Math|Vector|MakeVector (Math|Random|RandomFloatinRange (- (.X (Math|Vector|BreakVector (Spline|GetLocationatDistanceAlongSpline _spline (* _index _spacing) "World"))) 8e+01) (+ (.X (Math|Vector|BreakVector (Spline|GetLocationatDistanceAlongSpline _spline (* _index _spacing) "World"))) 5.0)) (Math|Random|RandomFloatinRange (- (.Y (Math|Vector|BreakVector (Spline|GetLocationatDistanceAlongSpline _spline (* _index _spacing) "World"))) 8e+01) (+ (.Y (Math|Vector|BreakVector (Spline|GetLocationatDistanceAlongSpline _spline (* _index _spacing) "World"))) 5.0)) (.Z (Math|Vector|BreakVector (Spline|GetLocationatDistanceAlongSpline _spline (* _index _spacing) "World"))))) "AlwaysSpawn" 0 0))
    (Variables|/Game/Blueprints/Mechanics/BP_Growflower.BP_Growflower_C|SetDestroy? _returnvalue false)
    (Effects|SpawnEmitteratLocation "/Game/Particles/Flowers/P_flowerSpawn.P_flowerSpawn" (Math|Vector|MakeVector (.X (Math|Vector|BreakVector (Spline|GetLocationatDistanceAlongSpline _spline (* _index _spacing) "World"))) (.Y (Math|Vector|BreakVector (Spline|GetLocationatDistanceAlongSpline _spline (* _index _spacing) "World"))) (+ (.Z (Math|Vector|BreakVector (Spline|GetLocationatDistanceAlongSpline _spline (* _index _spacing) "World"))) 7e+01)) "0, 0, 0" "2.000000,2.000000,2.000000" false)
    (Rendering|Components|Decal|SetFadeOut (Variables|Default|GetDecal) 0.0 2.0 false)
    (Utilities|IsValid _guidlightref
      (:Is%20Valid
        (Default|FlytoNextShrine _guidlightref)))))

(event EventBeginPlay
  (CallFunction|SpawnCollectorAlongSpline)
  (CallFunction|SpawnSplineMesh))

(event EventTick
  (params (DeltaSeconds :type Float%20%28single-precision%29))
  (Variables|Default|SetDeltaSeconds DeltaSeconds)
  (bind _asbp_save_variables (Utilities|Casting|CastToBP_SaveVariables (Game|GetGameInstance)))
  (Utilities|FlowControl|Sequence
    (:then_0
      (if (== (Variables|/Game/Blueprints/BP_SaveVariables.BP_SaveVariables_C|GetCollectorCount _asbp_save_variables) 1)
        (Utilities|FlowControl|DoOnce false
          (:Completed
            (bind _asbp_player (Utilities|Casting|CastToBP_Player (Game|Player|GetPlayerPawn 0)))
            (Variables|Default|SetSpherePosition (Transformation|GetWorldLocation (Variables|/Game/Blueprints/Player/BP_Player.BP_Player_C|GetHead _asbp_player)))))))
    (:then_1
      (if (== (Variables|/Game/Blueprints/BP_SaveVariables.BP_SaveVariables_C|GetCollectorCount _asbp_save_variables) (+ (Variables|Default|GetIndex) 1))
        (Transformation|SetRelativeLocation (Variables|Default|GetSphere) (Variables|Default|GetSpherePosition) false false)
        (if (Variables|Default|GetConected)
          (CallFunction|ShrineActivate)
          (Utilities|FlowControl|Delay 2.0)
          (Utilities|FlowControl|DoOnce false
            (:Completed
              (CallFunction|SpawnFlowersAlongSpline))))))))

(fn ConstructionScript)