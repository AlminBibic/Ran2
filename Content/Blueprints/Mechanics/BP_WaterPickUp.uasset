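; BP_WaterPickUp is a water pond pickup that grows the player on contact and then shrinks away.
; Overlapping its sphere with the player pawn calls AddBody and IncreasePulsPower on BP_Player and sets a shrinking flag.
; Tick interpolates the mesh scale down while flagged, with actor destruction gated on X scale dropping below zero.
; The construction script sets the mesh as the BPCDeformTerrain component's target.
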(event OnComponentBeginOverlap(OverlapSphere)
  (params (OverlappedComponent :type Primitive%20Component%20Object%20Reference) (OtherActor :type Actor%20Object%20Reference) (OtherComp :type Primitive%20Component%20Object%20Reference) (OtherBodyIndex :type Integer) (bFromSweep :type Boolean) (SweepResult :type Hit%20Result%20Structure%20%28by%20ref%29))
  (bind _returnvalue (Game|Player|GetPlayerPawn 0))
  ;[1 1 1] OnBeginOverlap with Player add a Body to Player
  (if (== OtherActor _returnvalue)
    (bind _asbp_player (Utilities|Casting|CastToBP_Player _returnvalue))
    (Default|AddBody _asbp_player)
    (Variables|Default|SetIsShrinking true)
    (Default|IncreasePulsPower _asbp_player)))

(event Custom|Shrink
  (bind _pickupmesh (Variables|Default|GetPickUpMesh))
  (bind _deltaseconds (Variables|Default|GetDeltaSeconds))
  (bind _shrinkspeed (Variables|Default|GetShrinkSpeed))
  (bind _returnvalue (Transformation|GetWorldScale _pickupmesh))
  (bind _returnvalue_2 (Math|Interpolation|FInterpTo (.x _returnvalue) 0.0 _deltaseconds _shrinkspeed))
  ;[1 1 1] Shrink the pond when overlapping with then Player
  (if (Variables|Default|GetIsShrinking)
    (Transformation|SetWorldScale3D _pickupmesh (Math|Vector|MakeVector _returnvalue_2 _returnvalue_2 (Math|Interpolation|FInterpTo (.z _returnvalue) 0.0 _deltaseconds _shrinkspeed)))
    (if (< (.x _returnvalue) 0.0)
      (Actor|DestroyActor))))

(event EventTick
  (params (DeltaSeconds :type Float%20%28single-precision%29))
  (Variables|Default|SetDeltaSeconds DeltaSeconds)
  (Utilities|FlowControl|Sequence
    (:then_0
      (CallFunction|Shrink))))

(fn ConstructionScript
  (|CallParentFunction)
  (Variables|/Game/Blueprints/Components/BPC_DeformTerrain.BPC_DeformTerrain_C|SetTarget (Variables|Default|GetBPC_DeformTerrain) (Variables|Default|GetPickUpMesh)))