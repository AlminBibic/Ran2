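; Connect-the-collectors shrine puzzle that spawns collectors at spline points, links them with spline meshes and opens a cliff when completed.
; An overlap sphere jumps to the first activated collector and completes the puzzle when the player enters it with the GameInstance count full.
; Completion lights the shrine, briefly switches camera, grows flowers and sends the guide light onward.
; Tick polls this state and eases the fill plane and cliff walls with VInterpTo.
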(event OnComponentBeginOverlap(Sphere)
  (params (OverlappedComponent :type Primitive%20Component%20Object%20Reference) (OtherActor :type Actor%20Object%20Reference) (OtherComp :type Primitive%20Component%20Object%20Reference) (OtherBodyIndex :type Integer) (bFromSweep :type Boolean) (SweepResult :type Hit%20Result%20Structure%20%28by%20ref%29))
  ;[1 1 1] Conected
  (if (== OtherActor (Game|Player|GetPlayerPawn 0))
    (bind _asbp_save_variables (Utilities|Casting|CastToBP_SaveVariables (Game|GetGameInstance)))
    (if (== (Variables|/Game/Blueprints/BP_SaveVariables.BP_SaveVariables_C|GetConnectCollerctorCount _asbp_save_variables) (+ (Variables|Default|GetIndex) 1))
      (Variables|Default|SetConected true))))

(event Custom|CheckFirstActivation
  ;[1 1 1] Check the first activation
  (for _array_element (Variables|BP_Collectors|GetBP_Collectors)
    (if (Variables|/Game/Blueprints/Mechanics/Connect/BP_ConnectCollect.BP_ConnectCollect_C|GetFirst _array_element)
      (Utilities|FlowControl|DoOnce false
        (:Completed
          (Transformation|SetWorldLocation (Variables|Default|GetSphere) (Transformation|GetActorLocation _array_element) false false))))))

(event Custom|ShrineActivate
  ;[1 1 1] ShrineActivate
  (Rendering|Material|SetScalarParameterValueonMaterials (Variables|Default|GetShrine) "Switch" 1.0)
  (Utilities|FlowControl|DoOnce false
    (:Completed
      (CallFunction|SwitchCamera))))

(event Custom|Shake
  (bind _wall_left (Variables|Default|GetWall_Left))
  (bind _wall_right (Variables|Default|GetWall_Right))
  ;[1 1 1] Shake
  (Transformation|SetRelativeLocation _wall_left (Math|Vector|MakeVector (Math|Random|RandomFloatinRange 0.0 2.0) (Math|Random|RandomFloatinRange 0.0 3.0) (.z (Variables|/Script/Engine.SceneComponent|GetRelativeLocation _wall_left))) false false)
  (Transformation|SetRelativeLocation _wall_right (Math|Vector|MakeVector (Math|Random|RandomFloatinRange 0.0 2.0) (Math|Random|RandomFloatinRange 0.0 3.0) (.z (Variables|/Script/Engine.SceneComponent|GetRelativeLocation _wall_right))) false false))

(event Custom|SpawnCollectorAlongSpline
  (bind _spline (Variables|Default|GetSpline))
  (bind _returnvalue (Spline|GetNumberOfSplinePoints _spline))
  (bind _returnvalue_2 (- _returnvalue 1))
  ;[1 1 1] Spawn Collector along Spline
  (Variables|Default|SetIndex _returnvalue_2)
  (for _index (range 0 _returnvalue_2)
    (bind _returnvalue_3 (Game|SpawnActorfromClass "/Game/Blueprints/Mechanics/Connect/BP_ConnectCollect.BP_ConnectCollect_C" (Math|Transform|MakeTransform (Spline|GetLocationatSplinePoint _spline _index "World")) "AlwaysSpawn" 0 0))
    (Utilities|Array|SetArrayElem (Variables|BP_Collectors|GetBP_Collectors) (Variables|Default|GetarrayIndex) _returnvalue_3 true)
    (Variables|Default|SetarrayIndex (+ (Variables|Default|GetarrayIndex) 1))))

(event Custom|SpawnSplineMesh
  (bind _spline (Variables|Default|GetSpline))
  ;[1 1 1] Create SplineMesh
  (for _index (range 1 (Spline|GetNumberOfSplinePoints (Variables|Default|GetSpline)))
    (bind _returnvalue (AddComponent|AddSplineMeshComponent true))
    (Variables|Default|SetSPM _returnvalue)
    (SplineMesh|SetStartandEnd _returnvalue (.Location (Spline|GetLocationandTangentatSplinePoint _spline (- _index 1) "World")) (.Tangent (Spline|GetLocationandTangentatSplinePoint _spline (- _index 1) "World")) (.Location (Spline|GetLocationandTangentatSplinePoint _spline _index "World")) (.Tangent (Spline|GetLocationandTangentatSplinePoint _spline _index "World")) true :!class /Script/Engine.SplineMeshComponent)))

(event Custom|SwitchCamera
  ;[1 1 1] CameraSwitch
  (Input|DisableInput (Game|GetPlayerController 0))
  (bind _asbp_player (Utilities|Casting|CastToBP_Player (Game|Player|GetPlayerPawn 0)))
  (Rendering|SetVisibility (Variables|/Game/Blueprints/Player/BP_Player.BP_Player_C|GetParticleSystem _asbp_player) false false)
  (Game|Player|SetViewTargetwithBlend (Game|GetPlayerController 0) (Variables|Default|GetCameraSwitch) (Variables|Default|GetCameraBlendTime) "VTBlend_Linear" 1.0 false)
  (Utilities|FlowControl|Delay (+ (Variables|Default|GetDelayToPlayer) (Variables|Default|GetCameraBlendTime)))
  (Game|Player|SetViewTargetwithBlend (Game|GetPlayerController 0) (Game|Player|GetPlayerPawn 0) (Variables|Default|GetCameraBlendTime) "VTBlend_Linear" 1.0 false)
  (Input|EnableInput (Game|GetPlayerController 0))
  (Rendering|SetVisibility (Variables|/Game/Blueprints/Player/BP_Player.BP_Player_C|GetParticleSystem _asbp_player) true false))

(event Custom|SpawnFlowersAlongSpline
  (bind _spline (Variables|Default|GetSpline))
  (bind _spacing (Variables|Default|GetSpacing))
  (bind _guidlightref (Variables|Default|GetGuidLightRef))
  ;[1 1 1] SpawnFlowersAlongSpline
  (for _index (range 0 (.ReturnValue (Math|Float|Division(WholeandRemainder) (Spline|GetSplineLength _spline) _spacing)))
    (Game|SpawnActorfromClass "/Game/Blueprints/Mechanics/BP_Growflower.BP_Growflower_C" (Math|Transform|MakeTransform (Math|Vector|MakeVector (Math|Random|RandomFloatinRange (- (.X (Math|Vector|BreakVector (Spline|GetLocationatDistanceAlongSpline _spline (* _index _spacing) "World"))) 8e+01) (+ (.X (Math|Vector|BreakVector (Spline|GetLocationatDistanceAlongSpline _spline (* _index _spacing) "World"))) 5.0)) (Math|Random|RandomFloatinRange (- (.Y (Math|Vector|BreakVector (Spline|GetLocationatDistanceAlongSpline _spline (* _index _spacing) "World"))) 8e+01) (+ (.Y (Math|Vector|BreakVector (Spline|GetLocationatDistanceAlongSpline _spline (* _index _spacing) "World"))) 5.0)) (.Z (Math|Vector|BreakVector (Spline|GetLocationatDistanceAlongSpline _spline (* _index _spacing) "World")))) (Math|Rotator|MakeRotator 0.0 0.0 (Math|Random|RandomFloatinRange 0.0 3.6e+02))) "AlwaysSpawn" 0 0)
    (Effects|SpawnEmitteratLocation "/Game/Particles/Flowers/P_flowerSpawn.P_flowerSpawn" (Math|Vector|MakeVector (.X (Math|Vector|BreakVector (Spline|GetLocationatDistanceAlongSpline _spline (* _index _spacing) "World"))) (.Y (Math|Vector|BreakVector (Spline|GetLocationatDistanceAlongSpline _spline (* _index _spacing) "World"))) (+ (.Z (Math|Vector|BreakVector (Spline|GetLocationatDistanceAlongSpline _spline (* _index _spacing) "World"))) 7e+01)) "0, 0, 0" "2.000000,2.000000,2.000000" false)
    (Rendering|Components|Decal|SetFadeOut (Variables|Default|GetDecal) 0.0 2.0 false)
    (Utilities|IsValid _guidlightref
      (:Is%20Valid
        (Default|FlytoNextShrine _guidlightref)))))

(event Custom|SpawnFlowersInSphereRadius
  (bind _spawnsphere (Variables|Default|GetSpawnSphere))
  (bind _returnvalue (Transformation|GetWorldLocation _spawnsphere))
  (bind _sphereradius (Variables|/Script/Engine.SphereComponent|GetSphereRadius _spawnsphere))
  (bind _returnvalue_2 (Math|Random|RandomPointinBoundingBox _returnvalue (Math|Vector|MakeVector _sphereradius _sphereradius 0.0)))
  (bind (_x _y _z) (Math|Vector|BreakVector _returnvalue_2))
  ;[1 1 1] Spawn Flowers in Sphere radius
  (for _index (range 0 50)
    (Game|SpawnActorfromClass "/Game/Blueprints/Mechanics/BP_Growflower.BP_Growflower_C" (Math|Transform|MakeTransform _returnvalue_2 (Math|Rotator|MakeRotator 0.0 0.0 (Math|Random|RandomFloatinRange 0.0 3.6e+02)) "1,1,1") "AlwaysSpawn" 0 0)
    (Effects|SpawnEmitteratLocation "/Game/Particles/Flowers/P_flowerSpawn.P_flowerSpawn" (Math|Vector|MakeVector _x _y (+ _z 7e+01)) "0, 0, 0" "2.000000,2.000000,2.000000" false)))

(event Custom|Fill
  (bind _plane (Variables|Default|GetPlane))
  ;[1 1 1] Fill
  (Transformation|SetRelativeLocation _plane (Math|Interpolation|VInterpTo (Variables|/Script/Engine.SceneComponent|GetRelativeLocation _plane) (Variables|Default|GetFillPlaneEndPos) (Variables|Default|GetDeltaSeconds) 0.5) false false))

(event Custom|SetCollectorsRotation
  ;[1 1 1] Set rotattions of the collectors/conectors
  (Utilities|FlowControl|Sequence
    (:then_0
      (Transformation|SetWorldRotation (Variables|/Script/Engine.Actor|GetRootComponent (Utilities|Array|Get(acopy) (Variables|BP_Collectors|GetBP_Collectors))) (Variables|BPCollectors|GetRotation_01) false false))
    (:then_1
      (Transformation|SetWorldRotation (Variables|/Script/Engine.Actor|GetRootComponent (Utilities|Array|Get(acopy) (Variables|BP_Collectors|GetBP_Collectors) 1)) (Variables|BPCollectors|GetRotation_02) false false))
    (:then_2
      (Transformation|SetWorldRotation (Variables|/Script/Engine.Actor|GetRootComponent (Utilities|Array|Get(acopy) (Variables|BP_Collectors|GetBP_Collectors) 2)) (Variables|BPCollectors|GetRotation_03) false false))))

(event Custom|DivideCilf
  (bind _wall_left (Variables|Default|GetWall_Left))
  (bind _wall_right (Variables|Default|GetWall_Right))
  ;[1 1 1] DivideCliff
  (if (Variables|Clif|GetDivideWall)
    (Transformation|SetRelativeLocation _wall_left (Math|Interpolation|VInterpTo (Variables|/Script/Engine.SceneComponent|GetRelativeLocation _wall_left) (Variables|Clif|GetClif_L_Pos) (Variables|Default|GetDeltaSeconds) 0.5) false true)
    (Transformation|SetRelativeLocation _wall_right (Math|Interpolation|VInterpTo (Variables|/Script/Engine.SceneComponent|GetRelativeLocation _wall_right) (Variables|Clif|GetClif_R_Pos) (Variables|Default|GetDeltaSeconds) 0.5) false true)))

(event EventBeginPlay
  (CallFunction|SpawnCollectorAlongSpline)
  (CallFunction|SpawnSplineMesh)
  (CallFunction|SetCollectorsRotation)
  (CallFunction|Fill))

(event EventTick
  (params (DeltaSeconds :type Float%20%28single-precision%29))
  (Variables|Default|SetDeltaSeconds DeltaSeconds)
  (Utilities|FlowControl|Sequence
    (:then_0
      (if (Variables|Default|GetConected)
        (CallFunction|Fill)))
    (:then_1
      (bind _asbp_save_variables (Utilities|Casting|CastToBP_SaveVariables (Game|GetGameInstance)))
      (Utilities|FlowControl|Sequence
        (:then_0
          (CallFunction|CheckFirstActivation))
        (:then_1
          (if (== (Variables|/Game/Blueprints/BP_SaveVariables.BP_SaveVariables_C|GetConnectCollerctorCount _asbp_save_variables) (+ (Variables|Default|GetIndex) 1))
            (if (Variables|Default|GetConected)
              (CallFunction|ShrineActivate)
              (Utilities|FlowControl|Delay 2.0)
              (Utilities|FlowControl|DoOnce false
                (:Completed
                  (CallFunction|SpawnFlowersAlongSpline)
                  (CallFunction|SpawnFlowersinSphereRadius)
                  (Variables|Clif|SetDivideWall true))))))))
    (:then_2
      (CallFunction|DivideCilf))))

(fn ConstructionScript)