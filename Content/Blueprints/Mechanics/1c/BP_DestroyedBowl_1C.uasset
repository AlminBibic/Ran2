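; BP_DestroyedBowl_1C is a bowl actor for the 1C mechanic that activates a shrine effect when the player first hits it.
; A DoOnce-gated mesh hit from the player pawn increments the 1C counter in the BP_SaveVariables game instance and sets a First flag.
; After a short delay, it flips the mesh material's Switch parameter and spawns an enlarged puff emitter at the mesh location.
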(event OnComponentHit(StaticMesh)
  (params (HitComponent :type Primitive%20Component%20Object%20Reference) (OtherActor :type Actor%20Object%20Reference) (OtherComp :type Primitive%20Component%20Object%20Reference) (NormalImpulse :type Vector :default "0, 0, 0") (Hit :type Hit%20Result%20Structure%20%28by%20ref%29))
  (if (== OtherActor (Game|Player|GetPlayerPawn 0))
    (Utilities|FlowControl|DoOnce false
      (:Completed
        (CallFunction|Count)
        (Variables|Default|SetFirst true)
        (CallFunction|ShrineActivate)))))

(event Custom|ShrineActivate
  ;[1 1 1] Shrine Activate
  (Utilities|FlowControl|Delay 2.0)
  (Rendering|Material|SetScalarParameterValueonMaterials (Variables|Default|GetStaticMesh) "Switch" 1.0)
  (Effects|SpawnEmitteratLocation "/Game/Particles/Flowers/P_Puff.P_Puff" (Transformation|GetWorldLocation (Variables|Default|GetStaticMesh)) "0, 0, 0" "7.000000,7.000000,7.000000" false))

(event Custom|Count
  (bind _asbp_save_variables (Utilities|Casting|CastToBP_SaveVariables (Game|GetGameInstance)))
  (Variables|/Game/Blueprints/BP_SaveVariables.BP_SaveVariables_C|Set1CCount _asbp_save_variables (+ (Variables|/Game/Blueprints/BP_SaveVariables.BP_SaveVariables_C|Get1CCount _asbp_save_variables) 1)))

(fn ConstructionScript)