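; BP_GlowStone is a glowing stone that the player activates by hitting it.
; The static mesh's hit event filters for the player pawn and runs once through a DoOnce.
; Activation switches on the glow through a "Switch" scalar material parameter, prints a debug message and calls CountStones on the referenced grow area.
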(event OnComponentHit(StaticMesh)
  (params (HitComponent :type Primitive%20Component%20Object%20Reference) (OtherActor :type Actor%20Object%20Reference) (OtherComp :type Primitive%20Component%20Object%20Reference) (NormalImpulse :type Vector :default "0, 0, 0") (Hit :type Hit%20Result%20Structure%20%28by%20ref%29))
  (if (== OtherActor (Game|Player|GetPlayerPawn 0))
    (Utilities|FlowControl|DoOnce false
      (:Completed
        (CallFunction|ActivateStone)
        (Development|PrintString "Activated Glowing Stone" true true "(R=0.994945,G=0.000000,B=1.000000,A=1.000000)")
        (Default|CountStones (Variables|Default|GetGrowAreaRef))))))

(event Custom|ActivateStone
  ;[1 1 1] Activete Stone
  (Rendering|Material|SetScalarParameterValueonMaterials (Variables|Default|GetStaticMesh) "Switch" 1.0))

(fn ConstructionScript)