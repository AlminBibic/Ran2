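; Grass decal actor that shrinks away once the player pawn enters its sphere trigger, accompanied by a brief camera cutaway.
; The construction script scales the decal by Radius, and Tick lowers that by RemoveSpeed per frame, independent of delta time, down to zero.
; As removal starts, a DoOnce disables player input, blends to CameraActor, waits, then starts blending back to the pawn and re-enables input.
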(event OnComponentBeginOverlap(Sphere)
  (params (OverlappedComponent :type Primitive%20Component%20Object%20Reference) (OtherActor :type Actor%20Object%20Reference) (OtherComp :type Primitive%20Component%20Object%20Reference) (OtherBodyIndex :type Integer) (bFromSweep :type Boolean) (SweepResult :type Hit%20Result%20Structure%20%28by%20ref%29))
  (if (== OtherActor (Game|Player|GetPlayerPawn 0))
    (Variables|GrassDecal|SetRemove true)))

(event Custom|SwitchCamera
  ;[1 1 1] Switch Camera
  (Input|DisableInput (Game|GetPlayerController 0))
  (Game|Player|SetViewTargetwithBlend (Game|GetPlayerController 0) (Variables|Camera|GetCameraActor) (Variables|Camera|GetBlendTime) "VTBlend_Linear" 1.0 false)
  (Utilities|FlowControl|Delay (+ (Variables|Camera|GetBlendTime) (Variables|Camera|GetDelayToPlayer)))
  (Game|Player|SetViewTargetwithBlend (Game|GetPlayerController 0) (Game|Player|GetPlayerPawn 0) (Variables|Camera|GetBlendTime) "VTBlend_Linear" 1.0 false)
  (Input|EnableInput (Game|GetPlayerController 0)))

(event Custom|RemoveDecal
  ;[1 1 1] Remove Decal
  (if (Variables|GrassDecal|GetRemove)
    (bind _output_get (Variables|GrassDecal|SetRadius (Math|Float|Clamp(Float) (- (Variables|GrassDecal|GetRadius) (Variables|GrassDecal|GetRemoveSpeed)) 0.0 (Variables|GrassDecal|GetRadius))))
    (Transformation|SetWorldScale3D (Variables|Default|GetDecal) (Math|Vector|MakeVector _output_get _output_get _output_get))
    (Utilities|FlowControl|DoOnce false
      (:Completed
        (CallFunction|SwitchCamera)))))

(event EventTick
  (params (DeltaSeconds :type Float%20%28single-precision%29))
  (Variables|Default|SetDeltaSeconds DeltaSeconds)
  (CallFunction|RemoveDecal))

(fn ConstructionScript
  (bind _radius (Variables|GrassDecal|GetRadius))
  ;[1 1 1] Set Decal size
  (Transformation|SetWorldScale3D (Variables|Default|GetDecal) (Math|Vector|MakeVector _radius _radius _radius)))