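; BP_Follower is an AI-driven follower that trails the player while its sphere hovers and wobbles.
; Each Tick measures the distance to the player's Head, setting Follow when it is at least 400 units away.
; While Follow is set, the AI controller moves toward the head's location; otherwise movement stops.
; Hover applies cosine-of-lifetime deltas, scaled by frame time, to the sphere's relative location and rotation.
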(event Custom|FollowPlayer
  (AI|Navigation|MovetoLocation (AI|GetAIController self) (Transformation|GetWorldLocation (Variables|/Game/Blueprints/Player/BP_Player.BP_Player_C|GetHead (Variables|Default|GetPlayer))) -1.0 false true false true 0))

(event Custom|CheckDistance
  (if (>= (Math|Vector|VectorLength (- (Transformation|GetActorLocation self) (Transformation|GetWorldLocation (Variables|/Game/Blueprints/Player/BP_Player.BP_Player_C|GetHead (Variables|Default|GetPlayer))))) 4e+02)
    (Variables|Default|SetFollow true)
    (else
      (Variables|Default|SetFollow false))))

(event Custom|Hover
  (bind _returnvalue (Actor|GetGameTimeSinceCreation))
  (bind _sphere (Variables|Default|GetSphere))
  (bind _deltaseconds (Variables|Default|GetDeltaSeconds))
  (bind _returnvalue_2 (Math|Trig|Cos(Radians) _returnvalue))
  (bind _returnvalue_3 (* _returnvalue_2 5.0))
  (bind _returnvalue_4 (* _returnvalue_2 1e+01))
  (bind _returnvalue_5 (* _returnvalue_2 15.0))
  (bind _returnvalue_6 (* (Math|Vector|MakeVector _returnvalue_4 _returnvalue_5 _returnvalue_3) _deltaseconds))
  (Transformation|AddRelativeLocation _sphere (* (Math|Vector|MakeVector (* _returnvalue_2 4e+01) (* _returnvalue_2 -15.0) (* _returnvalue_2 1e+01)) (Variables|Default|GetDeltaSeconds)) false false)
  (Transformation|AddRelativeRotation _sphere (Math|Rotator|MakeRotator (.x _returnvalue_6) (.y _returnvalue_6) (.z _returnvalue_6)) false false))

(event EventTick
  (params (DeltaSeconds :type Float%20%28single-precision%29))
  (Variables|Default|SetDeltaSeconds DeltaSeconds)
  (Utilities|FlowControl|Sequence
    (:then_0
      (CallFunction|CheckDistance))
    (:then_1
      (if (Variables|Default|GetFollow)
        (CallFunction|FollowPlayer)
        (else
          (AI|Navigation|StopMovement (Pawn|GetController)))))
    (:then_2
      (CallFunction|Hover))))

(fn ConstructionScript)