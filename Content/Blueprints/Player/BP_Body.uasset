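; BP_Body is a player body segment that trails the component ahead of it and knocks tree-tagged objects.
; SetFollowing takes the BodyEnd of the given PlayerHead as its target, and Tick moves the actor toward it with VInterpTo and teleport.
; Overlapping a tree-tagged component applies a forward velocity impulse after a short delay.
; BeginPlay sets Body visibility once from the player's ShowBodys flag.
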(event OnComponentBeginOverlap(Body)
  (params (OverlappedComponent :type Primitive%20Component%20Object%20Reference) (OtherActor :type Actor%20Object%20Reference) (OtherComp :type Primitive%20Component%20Object%20Reference) (OtherBodyIndex :type Integer) (bFromSweep :type Boolean) (SweepResult :type Hit%20Result%20Structure%20%28by%20ref%29))
  ;[1 1 1] Push Object when overlap
  (if (Components|ComponentHasTag OtherComp "Tree")
    (Utilities|FlowControl|Delay 0.35)
    (Physics|AddImpulse OtherComp (* (Math|Vector|GetForwardVector (Variables|Default|GetForwardDirection)) (Variables|Default|GetPower)) "None" true)))

(event Custom|PushForward
  ;[1 1 1] Push Body forward
  (Transformation|SetActorLocation (Math|Interpolation|VInterpTo (Transformation|GetActorLocation) (Transformation|GetWorldLocation (Variables|Default|GetBodyInFront)) (Variables|Default|GetDeltaSeconds) 5.0) false true))

(event Custom|SetFollowing
  (params (PlayerHead :type BP%20Player%20Object%20Reference))
  ;[1 1 1] SetFollowing
  (bind _output_get (Variables|Default|SetPlayerHead PlayerHead))
  (Variables|Default|SetBodyInFront (Variables|/Game/Blueprints/Player/BP_Player.BP_Player_C|GetBodyEnd _output_get)))

(event EventBeginPlay
  (bind _body (Variables|Default|GetBody))
  ;[1 1 1] Show/Hide Bodys (cant change in runtime)
  (bind _asbp_player (Utilities|Casting|CastToBP_Player (Game|Player|GetPlayerPawn 0)))
  (if (Variables|/Game/Blueprints/Player/BP_Player.BP_Player_C|GetShowBodys _asbp_player)
    (Development|SetHiddeninGame _body false false)
    (else
      (Development|SetHiddeninGame _body true false))))

(event EventTick
  (params (DeltaSeconds :type Float%20%28single-precision%29))
  (Variables|Default|SetDeltaSeconds DeltaSeconds)
  (Utilities|FlowControl|Sequence
    (:then_0
      (CallFunction|PushForward))))

(fn ConstructionScript
  (Variables|Default|SetCreate true))