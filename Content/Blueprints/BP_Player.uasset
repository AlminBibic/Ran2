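; Player Blueprint for a chained-body, snake-like character that moves by physics impulses on its Head.
; Each Tick pushes the Head along the Direction component's forward vector on forward input and steps its yaw for left/right input.
; BeginPlay constrains a spawned BP_Body to the Head; AddBody chains further segments, re-parenting SpawnPoint to the newest.
; Whirl is an empty stub, and the look-up lift logic is disconnected.
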(event Custom|Whirl
  (if (> (Input|AxisValues|GetWhirl) 0.0)
    _))

(event Custom|LookUp)

(event Custom|MoveForward
  (bind _movementspeed (Variables|Default|GetMovementSpeed))
  (bind _delataseconds (Variables|Default|GetDelataSeconds))
  (bind _returnvalue (* _delataseconds _movementspeed))
  ;[1 1 1] MoveForawrd
  (if (> (Math|Vector|VectorLength (* (Math|Vector|ClampVectorSize (Math|Vector|MakeVector (Input|AxisValues|GetMoveForward) 0.0 0.0) 0.0 1.0) _returnvalue)) 0.0)
    (Physics|AddImpulse (Variables|Default|GetHead) (* (Math|Vector|GetForwardVector (Variables|Default|GetDirection)) _returnvalue) "None" true)))

(event Custom|RotationRight
  ;[1 1 1] Rotation Left/Right
  (if (> (Input|AxisValues|GetMoveRight) 0.0)
    (Transformation|SetWorldRotation (Variables|Default|GetHead) (Math|Rotator|MakeRotator 0.0 0.0 (+ (.yaw (Transformation|GetWorldRotation (Variables|Default|GetHead))) (Variables|Default|GetRotationSpeed))) false false)))

(event Custom|RotationLeft
  ;[1 1 1] Rotation Left/Right
  (if (> (Input|AxisValues|GetMoveLeft) 0.0)
    (Transformation|SetWorldRotation (Variables|Default|GetHead) (Math|Rotator|MakeRotator 0.0 0.0 (- (.yaw (Transformation|GetWorldRotation (Variables|Default|GetHead))) (Variables|Default|GetRotationSpeed))) false false)))

(event Custom|AddBodyOnBeginPlay
  (bind _spawnpoint (Variables|Default|GetSpawnPoint))
  (bind _returnvalue (Transformation|GetWorldTransform _spawnpoint))
  ;[1 1 1] Add Body On BeginPlay
  (bind _returnvalue_2 (Game|SpawnActorfromClass "/Game/Blueprints/BP_Body.BP_Body_C" (Math|Transform|MakeTransform (.location _returnvalue) (Math|Rotator|MakeRotator (.roll (.rotation _returnvalue)) (.pitch (.rotation _returnvalue)) (.yaw (Transformation|GetWorldRotation (Variables|Default|GetHead)))) (.scale _returnvalue)) "AlwaysSpawn" 0 0))
  (Variables|Default|SetAttacheComponent (Variables|/Game/Blueprints/BP_Body.BP_Body_C|GetBody _returnvalue_2))
  (Class|PhysicsConstraintComponent|SetConstrainedComponents (Variables|/Game/Blueprints/BP_Body.BP_Body_C|GetContector _returnvalue_2) (Variables|Default|GetHead) "None" 0 "None")
  (CallFunction|ResetSpawnPoint))

(event Custom|AddBody
  (bind _spawnpoint (Variables|Default|GetSpawnPoint))
  (bind _returnvalue (Transformation|GetWorldTransform _spawnpoint))
  ;[1 1 1] AddBody
  (bind _returnvalue_2 (Game|SpawnActorfromClass "/Game/Blueprints/BP_Body.BP_Body_C" (Math|Transform|MakeTransform (.location _returnvalue) (Math|Rotator|MakeRotator (.roll (.rotation _returnvalue)) (.pitch (.rotation _returnvalue)) (.yaw (Transformation|GetWorldRotation (Variables|Default|GetAttacheComponent)))) (.scale _returnvalue)) "AlwaysSpawn" 0 0))
  (Class|PhysicsConstraintComponent|SetConstrainedComponents (Variables|/Game/Blueprints/BP_Body.BP_Body_C|GetContector _returnvalue_2) (Variables|Default|GetAttacheComponent) "None" 0 "None")
  (Variables|Default|SetAttacheComponent (Variables|/Game/Blueprints/BP_Body.BP_Body_C|GetBody _returnvalue_2))
  (CallFunction|ResetSpawnPoint))

(event EventBeginPlay
  (CallFunction|AddBodyonBeginPlay))

(event EventTick
  (params (DeltaSeconds :type Float%20%28single-precision%29))
  (Variables|Default|SetDelataSeconds DeltaSeconds)
  (Utilities|FlowControl|Sequence
    (:then_0
      (CallFunction|MoveForward))
    (:then_1
      (CallFunction|RotationLeft))
    (:then_2
      (CallFunction|RotationRight))
    (:then_3
      (CallFunction|Whirl))))

(fn ConstructionScript)

(fn ResetSpawnPoint
  (Transformation|AttachComponentToComponent (Variables|Default|GetSpawnPoint) (Variables|Default|GetAttacheComponent) "None" "KeepRelative" "KeepRelative" "KeepRelative" true))