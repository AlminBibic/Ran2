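; BP_Spiral is a construction-time Blueprint that lays copies of a mesh, described as stones, along a spline.
; The Construction Script divides the spline length by Spacing and adds a Static Mesh Component at each interval in local space, without following spline rotation.
; Each component takes the configured mesh, material and world scale.
; The event graph has no active logic.
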(event EventBeginPlay)

(event Collision|EventActorBeginOverlap
  (params (OtherActor :type Actor%20Object%20Reference)))

(event EventTick
  (params (DeltaSeconds :type Float%20%28single-precision%29)))

(fn ConstructionScript
  (bind _spline (Variables|Default|GetSpline))
  (bind _spacing (Variables|Spiral|GetSpacing))
  ;[1 1 1] Create stones along spline
  (for _index (range 0 (.ReturnValue (Math|Float|Division(WholeandRemainder) (Spline|GetSplineLength _spline) _spacing)))
    (bind _returnvalue (AddComponent|AddStaticMeshComponent false (Math|Transform|MakeTransform (Spline|GetLocationatDistanceAlongSpline _spline (* _index _spacing) "Local") "0.000000,0.000000, 0")))
    (Components|StaticMesh|SetStaticMesh _returnvalue (Variables|Spiral|GetMesh))
    (Rendering|Material|SetMaterial _returnvalue 0 (Variables|Spiral|GetMaterial))
    (Transformation|SetWorldScale3D _returnvalue (Variables|Spiral|GetScale))))