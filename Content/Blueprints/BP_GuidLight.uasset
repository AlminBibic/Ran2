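; BP_GuidLight is a guide light that moves its Sphere component toward the next shrine.
; Tick stores the frame's delta time for the custom FlyToNextShrine event to use.
; Each FlyToNextShrine call takes one VInterpTo step toward NextShrine's Shrine location at Speed, teleporting without sweep.
; Nothing in this Blueprint calls that event or sets the target shrine.
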(event Custom|FlyToNextShrine
  (bind _sphere (Variables|Default|GetSphere))
  (Transformation|SetWorldLocation _sphere (Math|Interpolation|VInterpTo (Transformation|GetWorldLocation _sphere) (Transformation|GetWorldLocation (Variables|/Game/Blueprints/Mechanics/Watering/BP_Watering.BP_Watering_C|GetShrine (Variables|Default|GetNextShrine))) (Variables|Default|GetDeltaSeconds) (Variables|Default|GetSpeed)) false true))

(event EventTick
  (params (DeltaSeconds :type Float%20%28single-precision%29))
  (Variables|Default|SetDeltaSeconds DeltaSeconds))

(fn ConstructionScript)