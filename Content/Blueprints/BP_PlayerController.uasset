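; Player controller for a level-select menu that lets a gamepad drive the mouse cursor.
; Each tick it reads four directional axis inputs and nudges the OS mouse position by CurserSpeed.
; MenuSelect checks per-level hover flags, currently only printing the level name.
; It also spawns a click particle on a fixed X plane at the Y/Z of the cursor trace hit.
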(event Custom|MouseCurserUp
  (bind _returnvalue (Game|GetPlayerController 0))
  (bind (_locationx _locationy) (Game|Player|GetMousePosition _returnvalue))
  ;[1 1 1] Mouse Curser Control with Gamepad
  ;;[1 1 1] MouseCurserUp
  (if (> (Input|AxisValues|GetMouseCurserUp) 0.0)
    (Class|PlayerController|SetMouseLocation (Game|GetPlayerController 0) (Math|Float|Truncate _locationx) (Math|Float|Truncate (- _locationy (Variables|Default|GetCurserSpeed))))))

(event Custom|MouseCurserDown
  (bind _returnvalue (Game|GetPlayerController 0))
  (bind (_locationx _locationy) (Game|Player|GetMousePosition _returnvalue))
  ;[1 1 1] Mouse Curser Control with Gamepad
  ;;[1 1 1] MouseCurserDown
  (if (> (Input|AxisValues|GetMouseCurserDown) 0.0)
    (Class|PlayerController|SetMouseLocation (Game|GetPlayerController 0) (Math|Float|Truncate _locationx) (Math|Float|Truncate (+ _locationy (Variables|Default|GetCurserSpeed))))))

(event Custom|MouseCurserRight
  (bind _returnvalue (Game|GetPlayerController 0))
  (bind (_locationx _locationy) (Game|Player|GetMousePosition _returnvalue))
  ;[1 1 1] Mouse Curser Control with Gamepad
  ;;[1 1 1] MouseCurserRight
  (if (> (Input|AxisValues|GetMouseCurserRight) 0.0)
    (Class|PlayerController|SetMouseLocation (Game|GetPlayerController 0) (Math|Float|Truncate (+ _locationx (Variables|Default|GetCurserSpeed))) (Math|Float|Truncate _locationy))))

(event Custom|MouseCurserLeft
  (bind _returnvalue (Game|GetPlayerController 0))
  (bind (_locationx _locationy) (Game|Player|GetMousePosition _returnvalue))
  ;[1 1 1] Mouse Curser Control with Gamepad
  ;;[1 1 1] MouseCurserLeft
  (if (> (Input|AxisValues|GetMouseCurserLeft) 0.0)
    (Class|PlayerController|SetMouseLocation (Game|GetPlayerController 0) (Math|Float|Truncate (- _locationx (Variables|Default|GetCurserSpeed))) (Math|Float|Truncate _locationy))))

(event Custom|CheckLevel01
  ;[1 1 1] Check Levels
  ;;[1 1 1] Check Level 01
  (if (Variables|Default|GetOnLevel01)
    (Development|PrintString "Level_01")))

(event Custom|CheckLevel02
  ;[1 1 1] Check Levels
  ;;[1 1 1] Check Level 02
  (if (Variables|Default|GetOnLevel02)
    (Development|PrintString "Level_02")))

(event Custom|CheckLevel03
  ;[1 1 1] Check Levels
  ;;[1 1 1] Check Level 03
  (if (Variables|Default|GetOnLevel03)
    (Development|PrintString "Level_03")))

(event EventTick
  (params (DeltaSeconds :type Float%20%28single-precision%29))
  (Utilities|FlowControl|Sequence
    (:then_0
      (CallFunction|MouseCurserDown))
    (:then_1
      (CallFunction|MouseCurserUp))
    (:then_2
      (CallFunction|MouseCurserRight))
    (:then_3
      (CallFunction|MouseCurserLeft))))

(event Input|ActionEvents|InputActionMenuSelect
  (params (Key :type Key%20Structure))
  ;[1 1 1] Menu Select
  (:Pressed
    (Utilities|FlowControl|Sequence
      (:then_0
        (CallFunction|CheckLevel01))
      (:then_1
        (CallFunction|CheckLevel02))
      (:then_2
        (CallFunction|CheckLevel03)))))

(event Input|ActionEvents|InputActionMenuSelect
  (params (Key :type Key%20Structure))
  (bind _hitresult (Game|Player|GetHitResultUnderCursorbyChannel "TraceTypeQuery2" true))
  (bind _location (Collision|BreakHitResult _hitresult))
  ;[0 1 0.03884] Spawn ripple effect on click
  (:Pressed
    (Effects|SpawnEmitteratLocation (Variables|Default|GetClickParticle) (Math|Vector|MakeVector -4e+01 (.y _location) (.z _location)) "0, 0, 0" "0.500000,0.500000,0.500000")))

(fn ConstructionScript)