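; BP_CaptrureActor is a scene capture actor that tracks grass-affecting objects around the player and feeds capture data to MPC_Grass.
; On BeginPlay it publishes the ortho width as CaptureSize and adds GrassAffector-tagged components on GrassAffector-tagged actors to the capture's show-only list.
; A fast looping timer runs MoveTarget, which follows PlayerRef in XY at fixed height and writes CaptureLocation to the parameter collection.
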(event EventBeginPlay
  (Rendering|Material|SetScalarParameterValue "/Game/Materials/Foliage/Grass/MPC_Grass.MPC_Grass" "CaptureSize" (Variables|/Script/Engine.SceneCaptureComponent2D|GetOrthoWidth (Variables|Default|GetSceneCaptureComponent2D)) :!class /Script/Engine.KismetMaterialLibrary)
  (Utilities|Time|SetTimerbyFunctionName 0 "MoveTarget" 0.01 true)
  (bind _outactors (Actor|GetAllActorswithTag "GrassAffector"))
  (for _array_element _outactors
    (for _array_element_2 (Actor|GetComponentsbyTag _array_element "/Script/Engine.PrimitiveComponent" "GrassAffector")
      (Rendering|SceneCapture|ShowOnlyComponent (Variables|Default|GetSceneCaptureComponent2D) _array_element_2))))

(fn ConstructionScript)

(fn MoveTarget
  (bind _playerref (Variables|Default|GetPlayerRef))
  (bind _returnvalue (Transformation|GetActorLocation _playerref))
  ;[1 1 1] MoveTarget
  (Transformation|SetActorLocation (Math|Vector|MakeVector (.x _returnvalue) (.y _returnvalue) (.z (Transformation|GetActorLocation))) false false)
  (Rendering|Material|SetVectorParameterValue "/Game/Materials/Foliage/Grass/MPC_Grass.MPC_Grass" "CaptureLocation" (Math|Conversions|ToLinearColor(Vector) (Transformation|GetActorLocation)) :!class /Script/Engine.KismetMaterialLibrary))