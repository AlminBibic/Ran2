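; Component that paints a terrain deformation mask into the RT_Terrain render target beneath a target component, every tick while DeformTerrain is enabled.
; A downward line trace from the target finds the hit point, which is normalized to UV space using the Landscape actor's origin and bounds.
; The DrawBrush material is then drawn onto the render target's canvas at that position, sized by DrawScale.
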(event Custom|Draw
  (bind _landscape (Variables|Terrain|GetLandscape))
  (bind _target (Variables|Default|GetTarget))
  (bind _landscape_2 (Variables|Terrain|GetLandscape))
  (bind _returnvalue (Transformation|GetWorldLocation _target))
  (bind _returnvalue_2 (Transformation|GetActorLocation _landscape))
  (bind _boxextent (Collision|GetActorBounds _landscape_2 false))
  ;[1 1 1] Draw to RenderTarget
  (bind _outhit (Collision|LineTraceByChannel (+ _returnvalue (Math|Vector|MakeVector 0.0 0.0 3e+01)) (- _returnvalue (Math|Vector|MakeVector 0.0 0.0 (Variables|Terrain|GetTraceDownAmount))) "TraceTypeQuery1" false 0 "None"))
  (bind (_canvas _size _context) (Rendering|BeginDrawCanvastoRenderTarget "/Game/Textures/RenderTarget/RT_Terrain.RT_Terrain"))
  (Canvas|DrawMaterial _canvas (Variables|Terrain|GetDrawBrush) (.Screen%20Position (CallFunction|SetCanvasMaterialScaleandPosition _size (Math|Vector2D|MakeVector2D (/ (Math|Float|Absolute(Float) (.x (- (Math|Vector2D|MakeVector2D (.x _returnvalue_2) (.y _returnvalue_2)) (Math|Vector2D|MakeVector2D (.x (.location _outhit)) (.y (.location _outhit)))))) (* (.x _boxextent) 2.0)) (/ (Math|Float|Absolute(Float) (.y (- (Math|Vector2D|MakeVector2D (.x _returnvalue_2) (.y _returnvalue_2)) (Math|Vector2D|MakeVector2D (.x (.location _outhit)) (.y (.location _outhit)))))) (* (.y _boxextent) 2.0))) (Variables|Terrain|GetDrawScale))) (.Screen%20Size (CallFunction|SetCanvasMaterialScaleandPosition _size (Math|Vector2D|MakeVector2D (/ (Math|Float|Absolute(Float) (.x (- (Math|Vector2D|MakeVector2D (.x _returnvalue_2) (.y _returnvalue_2)) (Math|Vector2D|MakeVector2D (.x (.location _outhit)) (.y (.location _outhit)))))) (* (.x _boxextent) 2.0)) (/ (Math|Float|Absolute(Float) (.y (- (Math|Vector2D|MakeVector2D (.x _returnvalue_2) (.y _returnvalue_2)) (Math|Vector2D|MakeVector2D (.x (.location _outhit)) (.y (.location _outhit)))))) (* (.y _boxextent) 2.0))) (Variables|Terrain|GetDrawScale))) "(X=0.000000,Y=0.000000)" "(X=1.000,Y=1.000)" 0.0 "(X=0.500000,Y=0.500000)")
  (Rendering|EndDrawCanvastoRenderTarget _context))

(event EventTick
  (params (DeltaSeconds :type Float%20%28single-precision%29))
  (if (Variables|Terrain|GetDeformTerrain)
    (CallFunction|Draw)))