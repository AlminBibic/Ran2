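; BP_LookAt is a one-shot trigger volume that briefly shifts the player's view to another camera target.
; When the player pawn first overlaps the box, it disables input, hides BP_Player's particle system and blends the view to CameraSwitch.
; After the blend time plus a configurable hold, it starts blending back, immediately restoring input and particles.
; The construction script sizes the box from the BoxExtent variable.
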(event OnComponentBeginOverlap(Box)
  (params (OverlappedComponent :type Primitive%20Component%20Object%20Reference) (OtherActor :type Actor%20Object%20Reference) (OtherComp :type Primitive%20Component%20Object%20Reference) (OtherBodyIndex :type Integer) (bFromSweep :type Boolean) (SweepResult :type Hit%20Result%20Structure%20%28by%20ref%29))
  (if (== OtherActor (Game|Player|GetPlayerPawn 0))
    (Utilities|FlowControl|DoOnce false
      (:Completed
        (CallFunction|Lookat)))))

(event Custom|LookAt
  ;[1 1 1] Look at
  (Input|DisableInput (Game|GetPlayerController 0))
  (bind _asbp_player (Utilities|Casting|CastToBP_Player (Game|Player|GetPlayerPawn 0)))
  (Rendering|SetVisibility (Variables|/Game/Blueprints/Player/BP_Player.BP_Player_C|GetParticleSystem _asbp_player) false false)
  (Game|Player|SetViewTargetwithBlend (Game|GetPlayerController 0) (Variables|Camera|GetCameraSwitch) (Variables|Camera|GetCameraBlendTime) "VTBlend_Linear" 1.0 false)
  (Utilities|FlowControl|Delay (+ (Variables|Camera|GetDelayToPlayer) (Variables|Camera|GetCameraBlendTime)))
  (Game|Player|SetViewTargetwithBlend (Game|GetPlayerController 0) (Game|Player|GetPlayerPawn 0) (Variables|Camera|GetCameraBlendTime) "VTBlend_Linear" 1.0 false)
  (Input|EnableInput (Game|GetPlayerController 0))
  (Rendering|SetVisibility (Variables|/Game/Blueprints/Player/BP_Player.BP_Player_C|GetParticleSystem _asbp_player) true false))

(fn ConstructionScript
  (Components|Box|SetBoxExtent (Variables|Default|GetBox) (Variables|CollisionBox|GetBoxExtent) true))